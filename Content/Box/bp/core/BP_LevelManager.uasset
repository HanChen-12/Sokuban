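; Level manager for a Sokoban box-pushing game that shows the main menu and runs levels, moves, undo and win checks.
; LoadLevel parses character rows from built-in or saved custom levels into a flat grid array, spawns tiles, boxes and player, and frames the orthographic camera.
; TryMove validates walks and pushes against that grid, stores capped position snapshots for UndoStep, and fires step and win notifications.
; Custom levels persist through a SaveGame slot.
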(event `self.ReceiveBeginPlay`
  (`self.LoadCustomLevels`)
  (bind _returnvalue (`|CreateWidget` "/Game/Box/bp/UI/WBP_MainMenu.WBP_MainMenu_C"))
  (`UserWidget.AddToViewport` _returnvalue 0))

(fn `AddNewLevel`
  (returns (NewIndex :type Integer))
  (return 0))

(fn `CheckWin`
  (for _array_element (`self.BoxActors`)
    (if (not (`self.IsGoal` (`/Game/Box/bp/actor/BP_Box.GridPos` _array_element)))
      (return)))
  (`self.OnWin`))

(fn `ClearLevel`
  (bind _playeractor (`self.PlayerActor`))
  (for _array_element (`self.TileActors`)
    (`self.K2_DestroyActor` _array_element))
  (for _array_element_2 (`self.BoxActors`)
    (`self.K2_DestroyActor` _array_element_2))
  (`/Engine/EditorBlueprintResources/StandardMacros.IsValid` _playeractor
    (:`Is Valid`
      (`self.K2_DestroyActor` _playeractor))
    (:`Is Not Valid`
      _))
  (`KismetArrayLibrary.Array_Clear` (`self.TileActors`))
  (`KismetArrayLibrary.Array_Clear` (`self.BoxActors`))
  (set `self.PlayerActor` null)
  (`KismetArrayLibrary.Array_Clear` (`self.GridData`))
  (`KismetArrayLibrary.Array_Clear` (`self.GoalSet`))
  (`KismetArrayLibrary.Array_Clear` (`self.UndoStack`)))

(fn `FindBoxAt`
  (params (P :type "IntPoint Structure"))
  (returns (ReturnValue :type "/Game/Box/bp/actor/BP_Box Object Reference"))
  (for _array_element (`self.BoxActors`)
    (bind _asbp_box (cast `/Game/Box/bp/actor/BP_Box` _array_element))
    (if (`KismetMathLibrary.Equal_IntPointIntPoint` (`/Game/Box/bp/actor/BP_Box.GridPos` _asbp_box) P)
      (return _array_element))))

(fn `GetGrid`
  (params (Col :type Integer) (Row :type Integer))
  (returns (ReturnValue :type "/Game/Box/bp/core/ETile Enum"))
  (return (`|GetArrayItem` (`self.GridData`) (+ Col (* Row (`self.GridCols`))))))

(fn `GetGridByIntPoint`
  (params (P :type "IntPoint Structure"))
  (returns (ReturnValue :type "/Game/Box/bp/core/ETile Enum"))
  (bind (_x _y) (break `IntPoint` P))
  (return (`self.GetGrid` _x _y)))

(fn `IsGoal`
  (params (P :type "IntPoint Structure"))
  (returns (ReturnValue :type Boolean))
  (return (`KismetArrayLibrary.Array_Contains` (`self.GoalSet`) P)))

(fn `LoadCustomLevels`
  (bind _returnvalue (`GameplayStatics.DoesSaveGameExist` "CustomLevels"))
  (if _returnvalue
    (bind _returnvalue_2 (`GameplayStatics.LoadGameFromSlot` "CustomLevels"))
    (bind _asbp_sokoban_save_game (cast `/Game/Box/bp/core/BP_SokobanSaveGame` _returnvalue_2))
    (set `self.CustomLevelDataList` (`/Game/Box/bp/core/BP_SokobanSaveGame.CustomLevels` _asbp_sokoban_save_game))))

(fn `LoadLevel`
  (params (Index :type Integer))
  (locals (NewOrthoWidth :type "Float (double-precision)") (CenterX :type Integer) (CenterY :type Integer) (LevelString :type String) (TempRows :type "Array of String"))
  (bind _gridcols (`self.GridCols`))
  (bind _gridrows (`self.GridRows`))
  (bind _temprows (`local.TempRows`))
  (`self.ClearLevel`)
  (set `self.CurrentLevelIndex` Index)
  (if (>= Index (`self.DefaultLevelCount`))
    (set `self.CustomIndex` (- Index (`self.DefaultLevelCount`)))
    (set `local.LevelString` (`|GetArrayItem` (`self.CustomLevelDataList`) (`self.CustomIndex`)))
    (set `self.ParsedRows` (`KismetStringLibrary.ParseIntoArray` (`local.LevelString`) "\\n"))
    (set `local.TempRows` (`self.ParsedRows`))
    (else
      (set `self.StepCount` 0)
      (set `self.LevelData` (`|GetArrayItem` (`self.LevelList`) Index))
      (set `local.TempRows` (`/Game/Box/bp/core/DA_LevelBase.Rows` (`self.LevelData`)))
      (set `self.ParsedRows` (`local.TempRows`))
      (set `local.TempRows` (`self.ParsedRows`))))
  (set `self.GridRows` (`KismetArrayLibrary.Array_Length` _temprows))
  (set `self.MaxLen` 0)
  (for _array_element _temprows
    (set `self.MaxLen` (`KismetMathLibrary.Max` (`KismetStringLibrary.Len` _array_element) (`self.MaxLen`))))
  (set `self.GridCols` (`self.MaxLen`))
  (`KismetArrayLibrary.Array_Clear` (`self.GridData`))
  (for _ (range (* (`self.GridCols`) (`self.GridRows`)))
    (`KismetArrayLibrary.Array_Add` (`self.GridData`) "NewEnumerator2"))
  (for _index (range (`self.GridRows`))
    ; 内
    (for _index_2 (range (`self.GridCols`))
      (bind _output (`|GetArrayItem` (`KismetStringLibrary.GetCharacterArrayFromString` (`|GetArrayItem` (`local.TempRows`) _index)) _index_2))
      (if (`KismetStringLibrary.EqualEqual_StrStr` _output "#")
        (`self.SpawnTile` _index_2 _index "NewEnumerator1")
        (`self.SetGridByIntPoint` "NewEnumerator1" (make `IntPoint` _index_2 _index))
        (elif (`KismetStringLibrary.EqualEqual_StrStr` _output " ")
          (`self.SpawnTile` _index_2 _index "NewEnumerator2")
          (`self.SetGridByIntPoint` "NewEnumerator2" (make `IntPoint` _index_2 _index))
          (elif (`KismetStringLibrary.EqualEqual_StrStr` _output ".")
            (`self.SpawnTile` _index_2 _index "NewEnumerator3")
            (bind _intpoint (make `IntPoint` _index_2 _index))
            (`KismetArrayLibrary.Array_Add` (`self.GoalSet`) _intpoint)
            (`self.SetGridByIntPoint` "NewEnumerator2" _intpoint)
            (elif (`KismetStringLibrary.EqualEqual_StrStr` _output "$")
              (`self.SpawnTile` _index_2 _index "NewEnumerator2")
              (`self.SpawnBox` _index_2 _index)
              (`self.SetGridByIntPoint` "NewEnumerator4" (make `IntPoint` _index_2 _index))
              (elif (`KismetStringLibrary.EqualEqual_StrStr` _output "@")
                (`self.SpawnTile` _index_2 _index "NewEnumerator2")
                (`self.SpawnPlayer` _index_2 _index)
                (`self.SetGridByIntPoint` "NewEnumerator5" (make `IntPoint` _index_2 _index))
                (elif (`KismetStringLibrary.EqualEqual_StrStr` _output "*")
                  (`self.SpawnTile` _index_2 _index "NewEnumerator3")
                  (bind _intpoint_2 (make `IntPoint` _index_2 _index))
                  (`KismetArrayLibrary.Array_Add` (`self.GoalSet`) _intpoint_2)
                  (`self.SpawnBox` _index_2 _index true)
                  (`self.SetGridByIntPoint` "NewEnumerator4" _intpoint_2)
                  (elif (`KismetStringLibrary.EqualEqual_StrStr` _output "+")
                    (`self.SpawnTile` _index_2 _index "NewEnumerator3")
                    (bind _intpoint_3 (make `IntPoint` _index_2 _index))
                    (`KismetArrayLibrary.Array_Add` (`self.GoalSet`) _intpoint_3)
                    (`self.SpawnPlayer` _index_2 _index)
                    (`self.SetGridByIntPoint` "NewEnumerator5" _intpoint_3))))))))))
  (bind _output_get (set `self.NewOrthoWidth` (* (`KismetMathLibrary.Conv_IntToDouble` (* (`KismetMathLibrary.Max` (`self.GridCols`) (`self.GridRows`)) 100)) 1.25)))
  (bind _outactors (`GameplayStatics.GetAllActorsOfClass` "/Script/Engine.CameraActor"))
  (`CameraComponent.SetOrthoWidth` (`CameraActor.CameraComponent` (`|GetArrayItem` _outactors)) _output_get)
  (`self.OnStepChanged` 0)
  (bind _outactors_2 (`GameplayStatics.GetAllActorsOfClass` "/Game/Box/bp/BP_Player.BP_Player_C"))
  (bind _asbp_player (cast `/Game/Box/bp/BP_Player` (`|GetArrayItem` _outactors_2)))
  (`/Game/Box/bp/BP_Player.UnLockInput` _asbp_player)
  (set `local.CenterX` (/ (* _gridcols 100) 2))
  (set `local.CenterY` (/ (* _gridrows 100) 2))
  (set `local.NewOrthoWidth` (* (`KismetMathLibrary.Conv_IntToDouble` (* (`KismetMathLibrary.Max` _gridcols _gridrows) 100)) 2.0))
  (bind _outactors_3 (`GameplayStatics.GetAllActorsOfClass` "/Script/Engine.CameraActor"))
  (bind _output_2 (`|GetArrayItem` _outactors_3))
  (bind `_as摄像机actor` (cast `CameraActor` _output_2))
  (`self.K2_SetActorLocation` _output_2 (`KismetMathLibrary.MakeVector` (`KismetMathLibrary.Conv_IntToDouble` (`local.CenterX`)) (`KismetMathLibrary.Conv_IntToDouble` (`local.CenterY`)) (`KismetMathLibrary.Conv_IntToDouble` (* (* (`KismetMathLibrary.Max` (`self.GridRows`) (`self.GridCols`)) 100) 8))) false false)
  (`CameraComponent.SetOrthoWidth` (`CameraActor.CameraComponent` `_as摄像机actor`) (`local.NewOrthoWidth`)))

(fn `NextLevel`
  (bind _nextindex (`self.NextIndex`))
  (set `self.NextIndex` (+ (`self.CurrentLevelIndex`) 1))
  (if (`KismetArrayLibrary.Array_IsValidIndex` (`self.LevelList`) _nextindex)
    (`self.LoadLevel` _nextindex)))

(fn `PrintGridData`
  (locals (RowString :type String))
  (for _index (range (`self.GridRows`))
    (for _index_2 (range (`self.GridCols`))
      (switch `/Game/Box/bp/core/ETile` (`self.GetGrid` _index_2 _index)
        (:`NewEnumerator0`
          (set `local.RowString` (`KismetStringLibrary.Concat_StrStr` (`local.RowString`))))
        (:`NewEnumerator1`
          (set `local.RowString` (`KismetStringLibrary.Concat_StrStr` (`local.RowString`) "#")))
        (:`NewEnumerator2`
          (set `local.RowString` (`KismetStringLibrary.Concat_StrStr` (`local.RowString`) "  ")))
        (:`NewEnumerator3`
          (set `local.RowString` (`KismetStringLibrary.Concat_StrStr` (`local.RowString`) ".")))
        (:`NewEnumerator4`
          (set `local.RowString` (`KismetStringLibrary.Concat_StrStr` (`local.RowString`) "$")))
        (:`NewEnumerator5`
          (set `local.RowString` (`KismetStringLibrary.Concat_StrStr` (`local.RowString`) "@"))))))
  (set `local.RowString` (`KismetStringLibrary.Concat_StrStr` (`local.RowString`) "\\n")))

(fn `PushSnapshot`
  (`KismetArrayLibrary.Array_Clear` (`self.TempBoxGrids`))
  (for _array_element (`self.BoxActors`)
    (`KismetArrayLibrary.Array_Add` (`self.TempBoxGrids`) (`/Game/Box/bp/actor/BP_Box.GridPos` _array_element)))
  (`KismetArrayLibrary.Array_Add` (`self.UndoStack`) (make `/Game/Box/bp/core/FSokobanSnapshot` (`/Game/Box/bp/BP_Player.GridPos` (`self.PlayerActor`)) (`self.TempBoxGrids`)))
  (if (> (`KismetArrayLibrary.Array_Length` (`self.UndoStack`)) 50)
    (`KismetArrayLibrary.Array_Remove` (`self.UndoStack`))))

(fn `RestartLevel`
  (`self.LoadLevel` (`self.CurrentLevelIndex`)))

(fn `SaveCustomLevels`
  (bind _returnvalue (`GameplayStatics.CreateSaveGameObject` "/Game/Box/bp/core/BP_SokobanSaveGame.BP_SokobanSaveGame_C"))
  (set `/Game/Box/bp/core/BP_SokobanSaveGame.CustomLevels` (`self.CustomLevelDataList`) _returnvalue)
  (`GameplayStatics.SaveGameToSlot` _returnvalue "CustomLevels"))

(fn `SetGrid`
  (params (Col :type Integer) (Row :type Integer) (Tile :type "/Game/Box/bp/core/ETile Enum" :default "NewEnumerator0"))
  (`KismetArrayLibrary.Array_Set` (`self.GridData`) (+ Col (* Row (`self.GridCols`))) Tile))

(fn `SetGridByIntPoint`
  (params (Tile :type "/Game/Box/bp/core/ETile Enum" :default "NewEnumerator0") (P :type "IntPoint Structure"))
  (bind (_x _y) (break `IntPoint` P))
  (`self.SetGrid` _x _y Tile))

(fn `SpawnBox`
  (params (Col :type Integer) (Row :type Integer) (bOnGoal :type Boolean))
  (bind _returnvalue (`|SpawnActorFromClass` (`self.BoxClass`) (`KismetMathLibrary.MakeTransform` (`/Game/Box/bp/core/BFL_Grid.GridToWorld` (make `IntPoint` Col Row) 50.0)) "AlwaysSpawn" "MultiplyWithRoot" null null))
  (bind _asbp_box (cast `/Game/Box/bp/actor/BP_Box` _returnvalue))
  (`/Game/Box/bp/actor/BP_Box.InitBox` _asbp_box (make `IntPoint` Col Row) bOnGoal)
  (`KismetArrayLibrary.Array_Add` (`self.BoxActors`) _asbp_box))

(fn `SpawnPlayer`
  (params (Col :type Integer) (Row :type Integer))
  (bind _returnvalue (`GameplayStatics.GetPlayerController` 0))
  (bind _returnvalue_2 (`|SpawnActorFromClass` (`self.PlayerClass`) (`KismetMathLibrary.MakeTransform` (`/Game/Box/bp/core/BFL_Grid.GridToWorld` (make `IntPoint` Col Row) 60.0)) "AlwaysSpawn" "MultiplyWithRoot" null null))
  (bind _asbp_player (cast `/Game/Box/bp/BP_Player` _returnvalue_2))
  (`/Game/Box/bp/BP_Player.InitPlayer` _asbp_player (make `IntPoint` Col Row) self)
  (set `self.PlayerActor` _asbp_player)
  (`Controller.Possess` _returnvalue (`self.PlayerActor`))
  (bind _outactors (`GameplayStatics.GetAllActorsOfClass` "/Script/Engine.CameraActor"))
  (`PlayerController.SetViewTargetWithBlend` _returnvalue (`|GetArrayItem` _outactors) 0.0 "VTBlend_Linear" 0.0 true))

(fn `SpawnTile`
  (params (Col :type Integer) (Row :type Integer) (TileType :type "/Game/Box/bp/core/ETile Enum" :default "NewEnumerator0"))
  (locals (NewLocalVar :type "Transform Structure"))
  (bind _returnvalue (`|SpawnActorFromClass` (`self.TileClass`) (`KismetMathLibrary.MakeTransform` (`/Game/Box/bp/core/BFL_Grid.GridToWorld` (make `IntPoint` Col Row))) "AlwaysSpawn" "MultiplyWithRoot" null null))
  (bind _asbp_tile (cast `/Game/Box/bp/actor/BP_Tile` _returnvalue))
  (`/Game/Box/bp/actor/BP_Tile.InitTile` _asbp_tile TileType)
  (`KismetArrayLibrary.Array_Add` (`self.TileActors`) _asbp_tile))

(fn `TryMove`
  (params (Direction :type "IntPoint Structure"))
  (returns (ReturnValue :type Boolean))
  (locals (Player :type "/Game/Box/bp/BP_Player Object Reference") (PlayerGrid :type "IntPoint Structure") (BehindTile :type "/Game/Box/bp/core/ETile Enum") (FoundBox :type "/Game/Box/bp/actor/BP_Box Object Reference"))
  (bind _behindgrid (`self.BehindGrid`))
  (set `local.PlayerGrid` (`/Game/Box/bp/BP_Player.GridPos` (`self.PlayerActor`)))
  (set `self.TargetGrid` (+ (`local.PlayerGrid`) Direction))
  (if (not (`/Game/Box/bp/core/BFL_Grid.IsValidGrid` (`self.TargetGrid`) (`self.GridCols`) (`self.GridRows`)))
    (return false)
    (else
      (set `self.TargetTile` (`self.GetGridByIntPoint` (`self.TargetGrid`)))
      (if (`|EnumEquality` (`self.TargetTile`) "NewEnumerator1")
        (return false)
        (else
          (if (`|EnumEquality` (`self.TargetTile`) "NewEnumerator4")
            (set `self.BehindGrid` (+ (`self.TargetGrid`) Direction))
            (if (not (`/Game/Box/bp/core/BFL_Grid.IsValidGrid` (`self.BehindGrid`) (`self.GridCols`) (`self.GridRows`)))
              (return false)
              (else
                (set `local.BehindTile` (`self.GetGridByIntPoint` (`self.BehindGrid`)))
                (if (or (`|EnumEquality` (`local.BehindTile`) "NewEnumerator1") (`|EnumEquality` (`local.BehindTile`) "NewEnumerator4"))
                  (return false)
                  (else
                    (`self.PushSnapshot`)
                    (bind _returnvalue (`self.FindBoxAt` (`self.TargetGrid`)))
                    (bind _output_get (set `local.FoundBox` _returnvalue))
                    (`self.SetGridByIntPoint` "NewEnumerator4" (`self.BehindGrid`))
                    (`self.SetGridByIntPoint` "NewEnumerator2" (`self.TargetGrid`))
                    (`/Game/Box/bp/actor/BP_Box.MoveToGrid` (`local.FoundBox`) _behindgrid (`self.IsGoal` _behindgrid))))))
            (else
              (`self.PushSnapshot`)))
          (`self.SetGridByIntPoint` "NewEnumerator2" (`local.PlayerGrid`))
          (`self.SetGridByIntPoint` "NewEnumerator5" (`self.TargetGrid`))
          (`/Game/Box/bp/BP_Player.MoveToGrid` (`self.PlayerActor`) (`self.TargetGrid`))
          (set `self.StepCount` (+ (`self.StepCount`) 1))
          (`self.OnStepChanged` (`self.StepCount`))
          (`self.CheckWin`)
          (return true))))))

(fn `UndoStep`
  (bind _boxgrid (`self.BoxGrid`))
  (bind (_playergrid _boxgrids) (break `/Game/Box/bp/core/FSokobanSnapshot` (`self.Snap`)))
  (bind _returnvalue (`KismetArrayLibrary.Array_LastIndex` (`self.UndoStack`)))
  (if (== (`KismetArrayLibrary.Array_Length` (`self.UndoStack`)) 0)
    (return)
    (else
      (set `self.Snap` (`|GetArrayItem` (`self.UndoStack`) _returnvalue))
      (`KismetArrayLibrary.Array_Remove` (`self.UndoStack`) _returnvalue)
      (for _index (range (`self.GridCols`))
        (for _index_2 (range (`self.GridRows`))
          (bind _returnvalue_2 (`self.GetGrid` _index _index_2))
          (if (or (`|EnumEquality` _returnvalue_2 "NewEnumerator5") (`|EnumEquality` _returnvalue_2 "NewEnumerator4"))
            (`self.SetGrid` _index _index_2 "NewEnumerator2"))))
      (`/Game/Box/bp/BP_Player.MoveToGrid` (`self.PlayerActor`) _playergrid)
      (`self.SetGridByIntPoint` "NewEnumerator5" _playergrid)
      (for _index_3 (range (`KismetArrayLibrary.Array_Length` (`self.BoxActors`)))
        (set `self.BoxGrid` (`|GetArrayItem` _boxgrids _index_3))
        (`/Game/Box/bp/actor/BP_Box.MoveToGrid` (`|GetArrayItem` (`self.BoxActors`) _index_3) _boxgrid (`self.IsGoal` _boxgrid))
        (`self.SetGridByIntPoint` "NewEnumerator4" _boxgrid))
      (bind _output_get (set `self.StepCount` (`KismetMathLibrary.Max` (- (`self.StepCount`) 1))))
      (`self.OnStepChanged` _output_get))))

(fn `UserConstructionScript`)