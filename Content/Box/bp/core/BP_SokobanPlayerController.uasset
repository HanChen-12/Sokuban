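; Player controller for a Sokoban box game that views the level through a fixed camera and enables mouse interaction.
; On BeginPlay it caches the first CameraActor in the level as the view target, shows the cursor, enables click events and sets Game and UI input.
; On possession it re-applies that camera as the view target, looking it up again if the cached reference is invalid.
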(event `self.ReceiveBeginPlay`
  (bind _outactors (`GameplayStatics.GetAllActorsOfClass` "/Script/Engine.CameraActor"))
  (bind `_as摄像机actor` (cast `CameraActor` (`|GetArrayItem` _outactors)))
  (bind _output_get (set `self.FixedCamera` `_as摄像机actor`))
  (`self.SetViewTargetWithBlend` self _output_get 0.0 "VTBlend_Linear" 0.0 true)
  (set `self.bShowMouseCursor` true)
  (set `self.bEnableClickEvents` true)
  (`WidgetBlueprintLibrary.SetInputMode_GameAndUIEx` null null "DoNotLock" false))

(event `self.ReceivePossess`
  (params (PossessedPawn :type "Pawn Object Reference"))
  (`/Engine/EditorBlueprintResources/StandardMacros.IsValid` (`self.FixedCamera`)
    (:`Is Valid`
      (`self.SetViewTargetWithBlend` self (`self.FixedCamera`) 0.0 "VTBlend_Linear" 0.0 true))
    (:`Is Not Valid`
      (bind _outactors (`GameplayStatics.GetAllActorsOfClass` "/Script/Engine.CameraActor"))
      (bind `_as摄像机actor` (cast `CameraActor` (`|GetArrayItem` _outactors)))
      (bind _output_get (set `self.FixedCamera` `_as摄像机actor`))
      (`self.SetViewTargetWithBlend` self _output_get 0.0 "VTBlend_Linear" 0.0 true))))

(fn `posses`)

(fn `UserConstructionScript`)