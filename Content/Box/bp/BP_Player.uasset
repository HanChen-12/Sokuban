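; BP_Player is the player pawn for a grid-based Sokoban puzzle, turning Enhanced Input actions into gameplay requests.
; Four-way moves, accepted only while not already moving, plus undo and restart are forwarded to the level manager supplied through InitPlayer.
; MoveToGrid updates the grid position and uses a timeline to interpolate the actor to the target cell.
; It also exposes input locking and a Back action that clears the level and opens the main menu.
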(event `self.ReceivePossessed`
  (params (NewController :type "Controller Object Reference")))

(event `self.ReceiveBeginPlay`
  (`KismetSystemLibrary.Delay` 0.2)
  (`EnhancedInputSubsystemInterface.AddMappingContext` (pcsubsystem `EnhancedInputLocalPlayerSubsystem` (`GameplayStatics.GetPlayerController` 0)) "/Game/Box/bp/Input/IMC_Sokoban.IMC_Sokoban" 0 (struct)))

(event `EnhancedInput|/Game/Box/bp/Input/IA_MoveUp`
  (params (ActionValue :type Boolean) (ElapsedSeconds :type "Float (double-precision)") (TriggeredSeconds :type "Float (double-precision)") (InputAction :type "InputAction Object Reference" :default "/Game/Box/bp/Input/IA_MoveUp.IA_MoveUp"))
  (:`Started`
    (if (not (`self.bIsMoving`))
      (`/Game/Box/bp/core/BP_LevelManager.TryMove` (`self.LevelManagerRef`) (make `IntPoint` 0 -1)))))

(event `EnhancedInput|/Game/Box/bp/Input/IA_MoveLeft`
  (params (ActionValue :type Boolean) (ElapsedSeconds :type "Float (double-precision)") (TriggeredSeconds :type "Float (double-precision)") (InputAction :type "InputAction Object Reference" :default "/Game/Box/bp/Input/IA_MoveLeft.IA_MoveLeft"))
  (:`Started`
    (if (not (`self.bIsMoving`))
      (`/Game/Box/bp/core/BP_LevelManager.TryMove` (`self.LevelManagerRef`) (make `IntPoint` -1)))))

(event `EnhancedInput|/Game/Box/bp/Input/IA_MoveRight`
  (params (ActionValue :type Boolean) (ElapsedSeconds :type "Float (double-precision)") (TriggeredSeconds :type "Float (double-precision)") (InputAction :type "InputAction Object Reference" :default "/Game/Box/bp/Input/IA_MoveRight.IA_MoveRight"))
  (:`Started`
    (if (not (`self.bIsMoving`))
      (`/Game/Box/bp/core/BP_LevelManager.TryMove` (`self.LevelManagerRef`) (make `IntPoint` 1)))))

(event `EnhancedInput|/Game/Box/bp/Input/IA_Undo`
  (params (ActionValue :type Boolean) (ElapsedSeconds :type "Float (double-precision)") (TriggeredSeconds :type "Float (double-precision)") (InputAction :type "InputAction Object Reference" :default "/Game/Box/bp/Input/IA_Undo.IA_Undo"))
  (:`Started`
    (`/Game/Box/bp/core/BP_LevelManager.UndoStep` (`self.LevelManagerRef`))))

(event `EnhancedInput|/Game/Box/bp/Input/IA_MoveDown`
  (params (ActionValue :type Boolean) (ElapsedSeconds :type "Float (double-precision)") (TriggeredSeconds :type "Float (double-precision)") (InputAction :type "InputAction Object Reference" :default "/Game/Box/bp/Input/IA_MoveDown.IA_MoveDown"))
  (:`Started`
    (if (not (`self.bIsMoving`))
      (`/Game/Box/bp/core/BP_LevelManager.TryMove` (`self.LevelManagerRef`) (make `IntPoint` 0 1)))))

(event `EnhancedInput|/Game/Box/bp/Input/IA_Restart`
  (params (ActionValue :type Boolean) (ElapsedSeconds :type "Float (double-precision)") (TriggeredSeconds :type "Float (double-precision)") (InputAction :type "InputAction Object Reference" :default "/Game/Box/bp/Input/IA_Restart.IA_Restart"))
  (:`Started`
    (`/Game/Box/bp/core/BP_LevelManager.RestartLevel` (`self.LevelManagerRef`))))

(event `EnhancedInput|/Game/Box/bp/Input/IA_Back`
  (params (ActionValue :type Boolean) (ElapsedSeconds :type "Float (double-precision)") (TriggeredSeconds :type "Float (double-precision)") (InputAction :type "InputAction Object Reference" :default "/Game/Box/bp/Input/IA_Back.IA_Back"))
  (:`Started`
    (`self.Back`)))

(fn `Back`
  (bind _outactors (`GameplayStatics.GetAllActorsOfClass` "/Game/Box/bp/core/BP_LevelManager.BP_LevelManager_C"))
  (`/Game/Box/bp/core/BP_LevelManager.ClearLevel` (`|GetArrayItem` _outactors))
  (bind _foundwidgets (`WidgetBlueprintLibrary.GetAllWidgetsOfClass` null))
  (`Widget.RemoveFromParent` (`|GetArrayItem` _foundwidgets))
  (bind _returnvalue (`|CreateWidget` "/Game/Box/bp/UI/WBP_MainMenu.WBP_MainMenu_C"))
  (`UserWidget.AddToViewport` _returnvalue 0))

(fn `InitPlayer`
  (params (StartGrid :type "IntPoint Structure") (Manager :type "/Game/Box/bp/core/BP_LevelManager Object Reference"))
  (bind _output_get (set `self.GridPos` StartGrid))
  (`self.K2_SetActorLocation` (`/Game/Box/bp/core/BFL_Grid.GridToWorld` _output_get 60.0))
  (set `self.LevelManagerRef` Manager))

(fn `LockInput`
  (`self.DisableInput` (`GameplayStatics.GetPlayerController` 0)))

(fn `MoveToGrid`
  (params (NewGrid :type "IntPoint Structure"))
  (set `self.GridPos` NewGrid)
  (set `self.StartPos` (`self.K2_GetActorLocation`))
  (set `self.TargetPos` (`/Game/Box/bp/core/BFL_Grid.GridToWorld` NewGrid 60.0))
  (set `self.bIsMoving` true)
  (`TimelineComponent.PlayFromStart` (`self.MoveTimeline`)))

(fn `UnlockInput`
  (`self.EnableInput` (`GameplayStatics.GetPlayerController` 0)))

(fn `UserConstructionScript`)