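; BP_Tile is a grid tile actor for the Box game that appears as a Wall, Floor or Goal.
; InitTile switches on a TileType to set the mesh's scale and material, with walls full height and floors and goals flattened.
; InstanceEditable duplicates that switch and also stores TileType.
; The event graph and construction script are empty, so neither function is called within this Blueprint.
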(fn `InitTile`
  (params (TileType :type "/Game/Box/bp/core/ETile Enum" :default "NewEnumerator0"))
  (switch `/Game/Box/bp/core/ETile` TileType
    (:`NewEnumerator1`
      (`SceneComponent.SetWorldScale3D` (`self.MeshComp`) (1.0 1.0 1.0))
      (`PrimitiveComponent.SetMaterial` (`self.MeshComp`) 0 "/Game/Box/bp/materials/M_Wall.M_Wall"))
    (:`NewEnumerator2`
      (`SceneComponent.SetWorldScale3D` (`self.MeshComp`) (1.0 1.0 0.1))
      (`PrimitiveComponent.SetMaterial` (`self.MeshComp`) 0 "/Game/Box/bp/materials/M_Floor.M_Floor"))
    (:`NewEnumerator3`
      (`SceneComponent.SetWorldScale3D` (`self.MeshComp`) (1.0 1.0 0.1))
      (`PrimitiveComponent.SetMaterial` (`self.MeshComp`) 0 "/Game/Box/bp/materials/M_Goal.M_Goal"))))

(fn `InstanceEditable`
  (params (TileType :type "/Game/Box/bp/core/ETile Enum" :default "NewEnumerator0"))
  (bind _meshcomp (`self.MeshComp`))
  (bind _output_get (set `self.TileType` TileType))
  (switch `/Game/Box/bp/core/ETile` _output_get
    (:`NewEnumerator1`
      (`SceneComponent.SetWorldScale3D` _meshcomp (1.0 1.0 1.0))
      (`PrimitiveComponent.SetMaterial` _meshcomp 0 "/Game/Box/bp/materials/M_Wall.M_Wall"))
    (:`NewEnumerator2`
      (`SceneComponent.SetWorldScale3D` _meshcomp (1.0 1.0 0.1))
      (`PrimitiveComponent.SetMaterial` _meshcomp 0 "/Game/Box/bp/materials/M_Floor.M_Floor"))
    (:`NewEnumerator3`
      (`SceneComponent.SetWorldScale3D` _meshcomp (1.0 1.0 0.1))
      (`PrimitiveComponent.SetMaterial` _meshcomp 0 "/Game/Box/bp/materials/M_Goal.M_Goal"))))

(fn `UserConstructionScript`)