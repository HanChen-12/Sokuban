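; BP_Box is a grid-placed box actor, apparently for a Sokoban-style puzzle, that shows by color whether it sits on a goal.
; InitBox snaps it to its starting cell, while MoveToGrid records the new cell and plays MoveTimeline to lerp it there.
; Both call UpdateColor, which creates a dynamic M_Box instance each time and tints it green on goal, orange otherwise.
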(fn `InitBox`
  (params (StartGrud :type "IntPoint Structure") (bOnGoal :type Boolean))
  (set `self.GridPos` StartGrud)
  (`self.K2_SetActorLocation` (`/Game/Box/bp/core/BFL_Grid.GridToWorld` StartGrud 50.0))
  (`self.UpdateColor` bOnGoal))

(fn `MoveToGrid`
  (params (NewGrid :type "IntPoint Structure") (bOnGoal :type Boolean))
  (set `self.GridPos` NewGrid)
  (set `self.StartPos` (`self.K2_GetActorLocation`))
  (set `self.TargetPos` (`/Game/Box/bp/core/BFL_Grid.GridToWorld` NewGrid 50.0))
  (`TimelineComponent.PlayFromStart` (`self.MoveTimeline`))
  (`self.UpdateColor` bOnGoal))

(fn `UpdateColor`
  (params (bOnGoal :type Boolean))
  (bind _staticmesh (`self.StaticMesh`))
  (bind _dynmaterial (`self.DynMaterial`))
  (bind _returnvalue (`PrimitiveComponent.CreateDynamicMaterialInstance` _staticmesh 0 "/Game/Box/bp/materials/M_Box.M_Box" "None"))
  (bind _output_get (set `self.DynMaterial` _returnvalue))
  (`PrimitiveComponent.SetMaterial` _staticmesh 0 _output_get)
  (if bOnGoal
    (`MaterialInstanceDynamic.SetVectorParameterValue` _dynmaterial "color" (struct :`G` 0.6 :`B` 0.2 :`A` 1.0))
    (else
      (`MaterialInstanceDynamic.SetVectorParameterValue` _dynmaterial "color" (struct :`R` 0.8 :`G` 0.4 :`B` 0.1 :`A` 1.0)))))

(fn `UserConstructionScript`)